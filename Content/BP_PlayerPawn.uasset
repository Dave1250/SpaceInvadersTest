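; BP_PlayerPawn is the player pawn, and its Blueprint logic handles the pause menu display.
; The game-paused event creates a WBP_Pause widget, adds it to the viewport, stores it and shows the mouse cursor.
; The unpaused event removes the stored widget and hides the cursor if that widget is still valid.
; BeginPlay and the construction script are empty.
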(event EventBeginPlay)

(event EventEffectonGamePaused
  (bind _returnvalue (UserInterface|CreateWidget "/Game/UI/WBP_Pause.WBP_Pause_C" (Game|GetPlayerController 0)))
  (UserInterface|Viewport|AddtoViewport _returnvalue 0)
  (Variables|Default|SetPauseWidget _returnvalue)
  (Variables|/Script/Engine.PlayerController|SetbShowMouseCursor (Game|GetPlayerController 0) true))

(event EventEffectonGameUnpaused
  (bind _pausewidget (Variables|Default|GetPauseWidget))
  (Utilities|IsValid _pausewidget
    (:Is%20Valid
      (Widget|RemovefromParent _pausewidget)
      (Variables|/Script/Engine.PlayerController|SetbShowMouseCursor (Game|GetPlayerController 0) false))))

(fn ConstructionScript)